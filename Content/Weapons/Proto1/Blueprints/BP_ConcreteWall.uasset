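; BP_ConcreteWall is a breakable concrete wall that gives way after a random number of hits, rolled at BeginPlay.
; Each ConcreteHit event counts a shot and applies localized external strain to ConcreteGeometry at the hit location, without propagation.
; At the threshold it marks itself broken, hides ConcreteMesh and disables that mesh's collision, ignoring further hits.
; Debug strings report damage and destruction.
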(event Custom|Concrete%20Hit
  (params (Hit%20Location :type Vector))
  (bind _concretemesh (Variables|Default|GetConcreteMesh))
  (if (not (Variables|Default|GetIsBroken))
    (bind _output_get (Variables|Default|SetShotsTaken (+ (Variables|Default|GetShotsTaken) 1)))
    (Class|GeometryCollectionComponent|ApplyExternalStrain (Variables|Default|GetConcreteGeometry) -1 Hit%20Location 15.0 0 0.0 5.5e+05)
    (if (>= _output_get (Variables|Default|GetShotsToBreak))
      (Variables|Default|SetIsBroken true)
      (Development|PrintString "Concrete Destroyed")
      (Rendering|SetVisibility _concretemesh false false)
      (Collision|SetCollisionEnabled _concretemesh "NoCollision")
      (else
        (Development|PrintString "Concrete Damaged")))))

(event EventBeginPlay
  (Variables|Default|SetShotsToBreak (Math|Random|RandomIntegerinRange 4 8)))

(event Collision|EventActorBeginOverlap
  (params (OtherActor :type Actor%20Object%20Reference)))

(event EventTick
  (params (DeltaSeconds :type Float%20%28single-precision%29)))

(fn ConstructionScript)