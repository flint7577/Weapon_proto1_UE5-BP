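; BP_ProtoProjectile is a prototype weapon projectile that damages enemy NPCs and penetrates certain tagged materials, with a short lifespan.
; On overlap it ignores the first-person character and damages BP_EnemyNPC without being destroyed.
; It passes through ProtoWood and one ProtoKevlar overlap, which sets HardMaterialPenetrated; once that is set, further wood or Kevlar destroys it.
; Any other actor destroys it immediately.
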(event EventBeginPlay
  (Actor|SetLifeSpan 2.0))

(event Collision|EventActorBeginOverlap
  (params (OtherActor :type Actor%20Object%20Reference))
  (Utilities|Casting|CastToBP_FirstPersonCharacter OtherActor
    (:CastFailed
      (bind _asbp_enemy_npc (Utilities|Casting|CastToBP_EnemyNPC OtherActor)
        (:then
          (Game|Damage|ApplyDamage _asbp_enemy_npc 1.0 0 0))
        (:CastFailed
          (if (Actor|ActorHasTag OtherActor "ProtoWood")
            (if (Variables|Default|GetHardMaterialPenetrated)
              (Actor|DestroyActor))
            (elif (Actor|ActorHasTag OtherActor "ProtoKevlar")
              (if (Variables|Default|GetHardMaterialPenetrated)
                (Actor|DestroyActor)
                (else
                  (Variables|Default|SetHardMaterialPenetrated true)))
              (else
                (Actor|DestroyActor)))))))))

(fn ConstructionScript)