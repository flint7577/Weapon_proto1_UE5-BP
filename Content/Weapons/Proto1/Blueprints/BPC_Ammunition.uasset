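; BPC_Ammunition is an ammo pickup for the prototype first-person weapon.
; When BP_FirstPersonCharacter overlaps its sphere, it calls RefillAmmo on the BP_WeaponProto1 in the ProtoWeapon child actor, then destroys itself.
; A separate ConsumeAmmo function clears a Consumable flag and optionally destroys the owner, but its success return with AmmoCount is unwired, and the overlap logic never calls it.
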(event OnComponentBeginOverlap(Sphere)
  (params (OverlappedComponent :type Primitive%20Component%20Object%20Reference) (OtherActor :type Actor%20Object%20Reference) (OtherComp :type Primitive%20Component%20Object%20Reference) (OtherBodyIndex :type Integer) (bFromSweep :type Boolean) (SweepResult :type Hit%20Result%20Structure%20%28by%20ref%29))
  (bind _asbp_first_person_character (Utilities|Casting|CastToBP_FirstPersonCharacter OtherActor))
  (bind _asbp_weapon_proto_1 (Utilities|Casting|CastToBP_WeaponProto1 (Variables|/Script/Engine.ChildActorComponent|GetChildActor (Variables|/Game/FirstPerson/Blueprints/BP_FirstPersonCharacter.BP_FirstPersonCharacter_C|GetProtoWeapon _asbp_first_person_character))))
  (Default|RefillAmmo _asbp_weapon_proto_1)
  (Actor|DestroyActor))

(event EventBeginPlay)

(event Collision|EventActorBeginOverlap
  (params (OtherActor :type Actor%20Object%20Reference)))

(event EventTick
  (params (DeltaSeconds :type Float%20%28single-precision%29)))

(fn ConstructionScript)

(fn ConsumeAmmo
  (if (Variables|Default|GetConsumable)
    (Variables|Default|SetConsumable false)
    (if (Variables|Default|GetDestroyUsed)
      (Actor|DestroyActor (Components|GetOwner)))
    (else
      (return 0 false))))